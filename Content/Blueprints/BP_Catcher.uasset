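; BP_Catcher is an enemy that roams randomly and chases the player on sight, marking itself Caught when it reaches them.
; PawnSensing starts an AI move toward the player and plays chase audio once per chase, while a retriggerable delay clears sight after a second.
; Tick uses delays to end the chase and fade audio after lost sight, and to pick random reachable roam points when not chasing.
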(event `self.ReceiveBeginPlay`
  ;[1 1 1] Create Audio Reference
  (bind _returnvalue (`AddComponent|NODE_AddAudioComponent-0`))
  (`AudioComponent.Stop` _returnvalue)
  (set `self.Audio` _returnvalue))

(event `self.PawnSensing.OnSeePawn`
  (params (Pawn :type "Pawn Object Reference"))
  ;[1 1 1] Chase
  (bind _ascoin_player_bp (cast `/Game/Blueprints/CoinPlayer_BP` (`GameplayStatics.GetPlayerCharacter` 0)))
  (if (not (`self.Caught`))
    (`|ExecutionSequence`
      (:`then_0`
        (set `self.CanSeePlayer` true)
        (set `self.IsChasing` true)
        (`|AIMoveTo` self (0.0 0.0 0.0) _ascoin_player_bp 2.0
          (:`then`
            (`/Engine/EditorBlueprintResources/StandardMacros.DoOnce` false :!label _label
              (:`Completed`
                (`AudioComponent.Play` (`self.Audio`) 0.0))))
          (:`OnSuccess`
            (set `self.Caught` true))))
      (:`then_1`
        (`KismetSystemLibrary.RetriggerableDelay` 1.0)
        (set `self.CanSeePlayer` false)))))

(event `self.ReceiveTick`
  (params (DeltaSeconds :type "Float (single-precision)"))
  ;[1 1 1] Chase
  (if (not (`self.Caught`))
    (`|ExecutionSequence`
      (:`then_0`
        (if (not (`self.CanSeePlayer`))
          (`KismetSystemLibrary.Delay` 4.0)
          (if (not (`self.CanSeePlayer`))
            (`AudioComponent.FadeOut` (`self.Audio`) 4.1 0.0 "Linear")
            (set `self.IsChasing` false)
            (goto _label :!via `Reset`))))
      (:`then_1`
        ;[1 1 1] Roam
        (if (not (`self.IsChasing`))
          (`KismetSystemLibrary.Delay` (`KismetMathLibrary.RandomFloatInRange` 2.0 5.0))
          (`|AIMoveTo` self (`NavigationSystemV1.K2_GetRandomReachablePointInRadius` (`self.K2_GetActorLocation`) 3000.0 null null) null))))))

(fn `UserConstructionScript`)